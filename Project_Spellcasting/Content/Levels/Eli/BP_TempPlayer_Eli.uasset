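; Temporary player character Blueprint with pause menu, HUD, walk toggle, nearest-actor attack and spell pickup.
; Health, stamina and death state live in CPPVitalsManager, with damage applied as negative healing and self-damage ignored.
; F takes a spell from the current container into MagicSystem's spellbook if the charge cap allows.
; Right-click release traces through the cached crosshair position and briefly swaps the hit static mesh's material, restoring it when a timeline finishes.
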(event `self.ReceiveBeginPlay`
  (`|ExecutionSequence`
    (:`then_0`
      ;[1 1 1] Create and Add Pause menu to viewport
      (bind _returnvalue (`|CreateWidget` "/Game/MainMenu/Menu.Menu_C"))
      (set `self.Pause Menu` _returnvalue))
    (:`then_1`
      ;[0.2 0.2 0.2] Add UI to viewport, and get crosshair's screen coordinates.
      (bind _returnvalue_2 (`|CreateWidget` "/Game/etc/UI.UI_C"))
      (`UserWidget.AddToViewport` _returnvalue_2 0)
      (bind _output_get (set `self.UI` _returnvalue_2))
      (`KismetSystemLibrary.Delay` 1.0) ; It needs some time to initialize or cache or smthn...
      (set `self.CrossHairPos` (`self.GetCrosshairPos` _output_get)))))

(event `Key|Escape`
  (params (Key :type "Key Structure"))
  ;[1 1 1] Create and Add Pause menu to viewport
  (:`Pressed`
    (`UserWidget.AddToViewport` (`self.Pause Menu`) 0)))

(event `Check If Dead`
  ;[1 1 1] Event Check Health
  (if (<= (`CPP_VitalsManagerComponent.CurrentHealth` (`self.CPP_VitalsManager`)) 0.0)
    (set `CPP_VitalsManagerComponent.bIsDead` true (`self.CPP_VitalsManager`))))

(event `self.Heal`
  (params (HealAmount :type "Float (single-precision)"))
  (bind _cpp_vitalsmanager (`self.CPP_VitalsManager`))
  (bind _cpp_vitalsmanager_2 (`self.CPP_VitalsManager`))
  (bind _returnvalue (+ HealAmount (`CPP_VitalsManagerComponent.CurrentHealth` _cpp_vitalsmanager)))
  ;[0.756 1 0.5916] Event Heal
  (if (> _returnvalue (`CPP_VitalsManagerComponent.MaxHealth` _cpp_vitalsmanager))
    (set `CPP_VitalsManagerComponent.CurrentHealth` (`CPP_VitalsManagerComponent.MaxHealth` _cpp_vitalsmanager_2) _cpp_vitalsmanager_2)
    (else
      (set `CPP_VitalsManagerComponent.CurrentHealth` _returnvalue (`self.CPP_VitalsManager`)))))

(event `self.UseStamina`
  (params (StaminaCost :type "Float (single-precision)"))
  (bind _cpp_vitalsmanager (`self.CPP_VitalsManager`))
  (bind _cpp_vitalsmanager_2 (`self.CPP_VitalsManager`))
  (bind _returnvalue (+ (`CPP_VitalsManagerComponent.CurrentStamina` _cpp_vitalsmanager) StaminaCost))
  ;[0.5594 1 0.9501] I'm tired
  (if (> _returnvalue (`CPP_VitalsManagerComponent.MaxStamina` _cpp_vitalsmanager))
    (set `CPP_VitalsManagerComponent.CurrentStamina` (`CPP_VitalsManagerComponent.MaxStamina` _cpp_vitalsmanager_2) _cpp_vitalsmanager_2)
    (else
      (set `CPP_VitalsManagerComponent.CurrentStamina` _returnvalue (`self.CPP_VitalsManager`)))))

(event `Key|LeftAlt`
  (params (Key :type "Key Structure"))
  (bind _charactermovement (`self.CharacterMovement`))
  ;[0.2 0.2 0.2] walk
  (:`Pressed`
    (set `CharacterMovementComponent.MaxWalkSpeed` 230.0 _charactermovement))
  (:`Released`
    (set `CharacterMovementComponent.MaxWalkSpeed` 500.0 _charactermovement)))

(event `Key|LeftMouseButton`
  (params (Key :type "Key Structure"))
  ;[0.2 0.2 0.2] fight
  (:`Pressed`
    (`/Game/etc/AC_Combat.Attack Nearest Actor` (`self.AC_Combat`))))

(event `Key|RightMouseButton`
  (params (Key :type "Key Structure"))
  ;[0.2 0.2 0.2] Get actor at crosshair, and highlight it.   (remember object's original material, change to another for half a sec, then reset to original)
  (:`Released`
    (`/Engine/EditorBlueprintResources/StandardMacros.IsValid` (`self.Mat`) ; null check
      (:`Is Not Valid`
        (bind (_hit _impactpoint _hitactor) (`self.LineTraceAtScreenPos` (`self.CrossHairPos`) 5000.0))
        (bind _asstatic_mesh_actor (cast `StaticMeshActor` _hitactor))
        (bind _staticmeshcomponent (`StaticMeshActor.StaticMeshComponent` _asstatic_mesh_actor))
        (set `self.Mat` (`PrimitiveComponent.GetMaterial` _staticmeshcomponent 0))
        (`PrimitiveComponent.SetMaterial` _staticmeshcomponent 0 "/Engine/VREditor/UI/ArrowMaterial.ArrowMaterial")
        (`Timeline|Timeline` :!via `PlayFromStart`
          (:`Finished`
            (`PrimitiveComponent.SetMaterial` _staticmeshcomponent 0 (`self.Mat`))
            (set `self.Mat` null) ; clear (for null check)
          ))))))

(event `self.RegenerateStamina`
  (params (StaminaAmount :type "Float (single-precision)")))

(event `self.ReceiveTick`
  (params (DeltaSeconds :type "Float (single-precision)"))
  ;[1 0 0.04606] Debug (TEMPORARY)
  ;;[1 1 1] Prints Current Spellbook amount on screen
)

(event `Key|F`
  (params (Key :type "Key Structure"))
  (bind _currentcontainertarget (`self.CurrentContainerTarget`))
  ;[1 0 0.04606] Debug (TEMPORARY)
  ;;[1 1 1] Gains a spell and puts in the Players Spellbook
  (:`Pressed`
    (if (`KismetSystemLibrary.IsValid` _currentcontainertarget)
      (bind _returnvalue (message `CPP_MagicSystemInterface.UseSpell` _currentcontainertarget))
      (`/Engine/EditorBlueprintResources/StandardMacros.IsValid` _returnvalue
        (:`Is Valid`
          (bind _returnvalue_2 (`self.GainSpell` _returnvalue))
          (if _returnvalue_2
            (`KismetSystemLibrary.PrintString` "Added 1 Spell!")))))))

(fn `ApplyDamage`
  (params (DamageInfo :type "DamageInfo Structure"))
  (returns (ReturnValue :type Boolean))
  (bind _returnvalue (and (not (`CPP_VitalsManagerComponent.bIsDead` (`self.CPP_VitalsManager`))) (!= DamageInfo_DamageCauser self)))
  (if _returnvalue
    (`self.Heal` (* DamageInfo_DamageAmount -1.0))
    (`self.Check If Dead`)
    (return _returnvalue)
    (else
      (return _returnvalue))))

(fn `GainSpell`
  (params (Spell :type "CPP_Spell Object Reference"))
  (returns (ReturnValue :type Boolean))
  (bind _returnvalue (`self.GetCharges`))
  (bind _returnvalue_2 (`self.GetMaximumCharges`))
  (bind _returnvalue_3 (+ _returnvalue (`CPP_Spell.SpellCharges` Spell)))
  (if (< _returnvalue_2 _returnvalue_3)
    (return false)
    (else
      (`KismetArrayLibrary.Array_Add` (`MagicSystemComponent.SpellBook` (`self.MagicSystem`)) Spell)
      (set `MagicSystemComponent.CurrentCharges` _returnvalue_3 (`self.MagicSystem`))
      (return true))))

(fn `GetCharges`
  (returns (ReturnValue :type "Float (single-precision)"))
  (return (`MagicSystemComponent.CurrentCharges` (`self.MagicSystem`))))

(fn `GetCurrentHealth`
  (returns (ReturnValue :type "Float (single-precision)"))
  (return (`CPP_VitalsManagerComponent.CurrentHealth` (`self.CPP_VitalsManager`))))

(fn `GetCurrentStamina`
  (returns (ReturnValue :type "Float (single-precision)"))
  (return (`CPP_VitalsManagerComponent.CurrentStamina` (`self.CPP_VitalsManager`))))

(fn `GetMaxHealth`
  (returns (ReturnValue :type "Float (single-precision)"))
  (return (`CPP_VitalsManagerComponent.MaxHealth` (`self.CPP_VitalsManager`))))

(fn `GetMaximumCharges`
  (returns (ReturnValue :type "Float (single-precision)"))
  (return (`MagicSystemComponent.MaxCharges` (`self.MagicSystem`))))

(fn `GetMaxStamina`
  (returns (ReturnValue :type "Float (single-precision)"))
  (return (`CPP_VitalsManagerComponent.MaxStamina` (`self.CPP_VitalsManager`))))

(fn `GetSpellType`
  (returns (ReturnValue :type "CPP_Spell Class Reference"))
  (return null))

(fn `IsBlocking`
  (returns (ReturnValue :type Boolean))
  (return (`CPP_VitalsManagerComponent.bIsBlocking` (`self.CPP_VitalsManager`))))

(fn `IsDead`
  (returns (ReturnValue :type Boolean))
  (return (`CPP_VitalsManagerComponent.bIsDead` (`self.CPP_VitalsManager`))))

(fn `LineTraceAtScreenPos`
  (params (ScreenPosition :type "Vector2D Structure (by ref)") (Range :type "Float (single-precision)"))
  (returns (Hit :type Boolean) (ImpactPoint :type "Vector Structure") (HitActor :type "Actor Object Reference"))
  (bind (_worldposition _worlddirection) (`GameplayStatics.DeprojectScreenToWorld` (`GameplayStatics.GetPlayerController` 0) ScreenPosition))
  (bind (_outhit _returnvalue) (`KismetSystemLibrary.LineTraceSingle` _worldposition (+ _worldposition (* _worlddirection Range)) "TraceTypeQuery1"))
  (bind (_bblockinghit _binitialoverlap _time _distance _location _impactpoint _normal _impactnormal _physmat _hitactor) (`GameplayStatics.BreakHitResult` _outhit))
  (return _returnvalue _impactpoint _hitactor))

(fn `OnRep_testvar`)

(fn `UserConstructionScript`)

(fn `UseSpell`
  (returns (ReturnValue :type "CPP_Spell Object Reference"))
  (return null))