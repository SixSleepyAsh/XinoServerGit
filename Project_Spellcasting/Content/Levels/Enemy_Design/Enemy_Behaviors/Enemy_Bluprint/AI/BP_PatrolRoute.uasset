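; BP_PatrolRoute is a spline-based patrol route that tracks which point an enemy AI is at.
; IncrementPatrolRoute steps PatrolIndex along the PatrolRoute spline points by PatrolDirection, which is 1 or -1.
; The direction flips on reaching the last or first point, so the route runs back and forth instead of looping.
; It only maintains the index and direction; it contains no movement logic.
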(event `Increment Patrol Route`
  ;[0.154 0.2668 1] This custom event increments the patrol route index, controlling the AI's movement along the spline.
  ; The Patrol Index is the current node the AI is at
  ; The Patrol Direction is the Direction they are moving in { 1 or -1 }
  (bind _output_get (set `self.PatrolIndex` (+ (`self.PatrolIndex`) (`self.PatrolDirection`))))
  ;;[0.01503 0.7068 1] Check if we've reached the end of the spline route. If so, change direction.
  (if (== _output_get (- (`SplineComponent.GetNumberOfSplinePoints` (`self.PatrolRoute`)) 1))
    (set `self.PatrolDirection` -1)
    (else
      ;;[1 0 0.01989] Check if we've reached the beginning of the spline route. If so, change direction again.
      (if (== (`self.PatrolIndex`) 0)
        (set `self.PatrolDirection` 1)))))

(fn `UserConstructionScript`)