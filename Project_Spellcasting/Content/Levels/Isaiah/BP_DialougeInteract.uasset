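; Interactable dialogue actor that shows an InteractIcon and allows talking while any actor overlaps it.
; Begin and end overlap toggle the icon and the CanTalk flag, with no check on which actor overlaps.
; E or left mouse print CanTalk and, if true, create a WBP_DialougeBox widget, which is not added to the viewport here.
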(event `self.ReceiveActorBeginOverlap`
  (params (OtherActor :type "Actor Object Reference"))
  (`SceneComponent.SetVisibility` (`self.InteractIcon`) true false)
  (set `self.CanTalk` true)
  (`KismetSystemLibrary.PrintString` "In range"))

(event `self.ReceiveActorEndOverlap`
  (params (OtherActor :type "Actor Object Reference"))
  (`SceneComponent.SetVisibility` (`self.InteractIcon`) false false)
  (set `self.CanTalk` false)
  (`KismetSystemLibrary.PrintString` "Left range"))

(event `Key|E`
  (params (Key :type "Key Structure"))
  (bind _cantalk (`self.CanTalk`))
  (:`Pressed`
    (`KismetSystemLibrary.PrintString` (`KismetStringLibrary.Conv_BoolToString` _cantalk) :!label _label)
    (if _cantalk
      (`|CreateWidget` "/Game/Levels/Isaiah/WBP_DialougeBox.WBP_DialougeBox_C"))))

(event `Key|LeftMouseButton`
  (params (Key :type "Key Structure"))
  (:`Pressed`
    (goto _label)))

(fn `UserConstructionScript`)