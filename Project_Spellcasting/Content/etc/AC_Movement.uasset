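; Movement component for a Character owner that adds a double jump and a timed dodge dash.
; Both launch along the last movement input by setting velocity directly and play the jump montage.
; The dash temporarily uses Flying mode, returns to Falling at walk speed, then waits out a cooldown.
; Both share the CanDJ flag, which gates air use and resets through a Landed delegate bound on use.
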(event `self.ReceiveBeginPlay`
  (`self.Init References`))

(event `EnhancedInput|/Game/ThirdPerson/Input/Actions/IA_Jump`
  (params (ActionValue :type Boolean) (ElapsedSeconds :type "Float (double-precision)") (TriggeredSeconds :type "Float (double-precision)") (InputAction :type "InputAction Object Reference" :default "/Game/ThirdPerson/Input/Actions/IA_Jump.IA_Jump"))
  (bind _character (`self.Character`))
  (:`Started`
    (if (and (`NavMovementComponent.IsFalling` (`Character.CharacterMovement` (`self.Character`))) (`self.CanDJ`))
      (`|PlayMontage` (`Character.Mesh` _character) "/Game/PlaceholderAnimations/MM_Jump_Montage.MM_Jump_Montage"
        (:`then`
          (set `MovementComponent.Velocity` (`self.DJ Velocity`) (`Character.CharacterMovement` _character))
          ;[0.2 0.2 0.2] Can't doublejump again until you land
          (set `self.CanDJ` false :!label _label)
          (add `Character.LandedDelegate` (`self.Character`) (delegate `Landed`)))))))

(event `Landed`
  (params (Hit :type "HitResult Structure (by ref)"))
  ;[0.2 0.2 0.2] Can't doublejump again until you land
  (set `self.CanDJ` true)
  (clear `Character.LandedDelegate` (`self.Character`)))

(event `EnhancedInput|/Game/ThirdPerson/Input/Actions/IA_Dodge`
  (params (ActionValue :type Boolean) (ElapsedSeconds :type "Float (double-precision)") (TriggeredSeconds :type "Float (double-precision)") (InputAction :type "InputAction Object Reference" :default "/Game/ThirdPerson/Input/Actions/IA_Dodge.IA_Dodge"))
  (bind _charactermovement (`Character.CharacterMovement` (`self.Character`)))
  (bind _charactermovement_2 (`Character.CharacterMovement` (`self.Character`)))
  (:`Started`
    (if (and (not (`self.Dashing`)) (or (not (`NavMovementComponent.IsFalling` (`Character.CharacterMovement` (`self.Character`)))) (`self.CanDJ`)))
      (set `self.Dashing` true)
      (`|PlayMontage` (`Character.Mesh` (`self.Character`)) "/Game/PlaceholderAnimations/MM_Jump_Montage.MM_Jump_Montage"
        (:`then`
          (`CharacterMovementComponent.SetMovementMode` _charactermovement_2 "MOVE_Flying" 0)
          (set `MovementComponent.Velocity` (`self.Dash Velocity` (/ (`self.Dash Distance`) (`self.Dash Duration`))) _charactermovement_2)
          ;[0.2 0.2 0.2] Reset from dashing
          (`KismetSystemLibrary.Delay` (`self.Dash Duration`))
          (`CharacterMovementComponent.SetMovementMode` _charactermovement "MOVE_Falling" 0)
          (`|ExecutionSequence`
            (:`then_0`
              (if (`NavMovementComponent.IsFalling` (`Character.CharacterMovement` (`self.Character`)))
                (goto _label)))
            (:`then_1`
              (set `MovementComponent.Velocity` (`self.Dash Velocity` (`CharacterMovementComponent.MaxWalkSpeed` _charactermovement)) _charactermovement)
              (`|PlayMontage` (`Character.Mesh` (`self.Character`)) "/Game/PlaceholderAnimations/MM_Jump_Montage.MM_Jump_Montage" 1000.0 ; stop current animation
                (:`then`
                  (`KismetSystemLibrary.Delay` (`self.Dash Cooldown`))
                  (set `self.Dashing` false))))))))))