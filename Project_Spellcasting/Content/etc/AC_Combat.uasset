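; Actor component that gives a Character melee combo attacks and a front flip over nearby enemies.
; Light attack picks the target best aligned with movement via box trace, preferring any blocker found by line trace, else strikes along the intended direction.
; Attacks, also callable by direction or location, cycle punch-punch-kick montages (kick when airborne) and feed Motion Warping's StrikeTarget.
; Jumping near a target plays the flip with capsule collision temporarily disabled.
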(event `Attack Nearest Actor`
  (`KismetSystemLibrary.PrintString` "Warning: \"Attack Nearest Actor\" event will be removed from AC_Combat. Please delete its references from other blueprings." true true (struct :`R` 1.0 :`G` 0.316363 :`A` 1.0) 5.0))

(event `self.ReceiveBeginPlay`
  (`self.Init References`))

(event `EnhancedInput|/Game/ThirdPerson/Input/Actions/IA_LightAttack`
  (params (ActionValue :type Boolean) (ElapsedSeconds :type "Float (double-precision)") (TriggeredSeconds :type "Float (double-precision)") (InputAction :type "InputAction Object Reference" :default "/Game/ThirdPerson/Input/Actions/IA_LightAttack.IA_LightAttack"))
  (:`Started`
    (if (not (`self.Attacking`))
      (bind (_target_found _closestactor _intendeddirection) (`self.Get Closest Targeted Actor` (`self.Dash Range`))) ; todo: line trace to make sure this one's closest
      ;[0.2 0.2 0.2 1 15] If found, attack target location (absolute)
      ; If not found, attack towards current movement direction (relative)
      (if _target_found
        (set `self.DashTarget` (`Actor.K2_GetActorLocation` _closestactor))
        (set `self.DashTargetRelative` false)
        (else
          (set `self.DashTarget` _intendeddirection)
          (set `self.DashTargetRelative` true)))
      (set `self.Attacking` true :!label _label)
      (`self.pExecute Attack`))))

(event `Attack`
  (params (`Dash Distance` :type "Float (double-precision)"))
  ;[0.2 0.2 0.2] Towards current movement direction (relative)
  (if (not (`self.Attacking`))
    (set `self.DashTargetRelative` true)
    (set `self.DashTarget` (`self.Determine Dash Target` `Dash Distance`))
    (goto _label)))

(event `Attack Location`
  (params (`Target Location` :type "Vector Structure"))
  ;[0.2 0.2 0.2] Specific location (absolute)
  (if (not (`self.Attacking`))
    (set `self.DashTargetRelative` false)
    (set `self.DashTarget` `Target Location`)
    (goto _label)))

(event `pExecute Attack`
  (bind _dashtarget (`self.DashTarget`))
  (set `self.AttackPending` false)
  (if (`NavMovementComponent.IsFalling` (`self.Movement`))
    (set `self.ComboCounter` 2))
  (`|PlayMontage` (`self.Mesh`) (select `int` (`self.ComboCounter`) :`0` "/Game/PlaceholderAnimations/Punch1_Montage.Punch1_Montage" :`1` "/Game/PlaceholderAnimations/Punch2_Montage.Punch2_Montage" :`2` "/Game/PlaceholderAnimations/Kick_Montage.Kick_Montage" :!type "AnimMontage Object Reference") ; Choose montage based on current combo counter
    (:`then`
      (set `self.ComboCounter` (`KismetMathLibrary.Wrap` (+ (`self.ComboCounter`) 1) -1 2)) ; increment or loop around
      (`MotionWarpingComponent.AddOrUpdateWarpTargetFromLocation` (`self.MotionWarping`) "StrikeTarget" (select `bool` (`self.DashTargetRelative`) :`false` _dashtarget :`true` (+ _dashtarget (`Actor.K2_GetActorLocation` (`self.Character`))))))
    (:`OnCompleted`
      (set `self.ComboCounter` 0) ; If a montage fully plays out, combo ends
    )
    (:`OnNotifyEnd`
      (set `self.Attacking` false) ; Able to attack again
    )))

(event `EnhancedInput|/Game/ThirdPerson/Input/Actions/IA_Jump`
  (params (ActionValue :type Boolean) (ElapsedSeconds :type "Float (double-precision)") (TriggeredSeconds :type "Float (double-precision)") (InputAction :type "InputAction Object Reference" :default "/Game/ThirdPerson/Input/Actions/IA_Jump.IA_Jump"))
  (bind _capsulecomponent (`Character.CapsuleComponent` (`self.Character`)))
  ;[0.2 0.2 0.2] Jump over enemy
  (:`Triggered`
    (`KismetSystemLibrary.DelayUntilNextTick`)
    (if (`Character.bWasJumping` (`self.Character`))
      (bind _target_found (`self.Get Closest Targeted Actor` 80.0))
      (if _target_found
        (`|PlayMontage` (`self.Mesh`) "/Game/PlaceholderAnimations/FrontFlip_Montage.FrontFlip_Montage"
          (:`then`
            (`PrimitiveComponent.SetCollisionEnabled` _capsulecomponent "NoCollision"))
          (:`OnBlendOut`
            (`KismetSystemLibrary.Delay` 0.1 :!label _label_2)
            (`PrimitiveComponent.SetCollisionEnabled` _capsulecomponent "QueryAndPhysics"))
          (:`OnInterrupted`
            (goto _label_2)))))))

(fn `Get Closest Targeted Actor`
  (params (Range :type "Float (single-precision)"))
  (returns (`Target Found` :type Boolean) (ClosestActor :type "Actor Object Reference") (IntendedDirection :type "Vector Structure"))
  (locals (Closeness :type "Float (double-precision)" :default 0.0) (Direction :type "Vector Structure" :default (0.0 0.0 0.0)) (`Closest Actor` :type "Actor Object Reference"))
  (bind (_location _tryingtomove) (`self.Determine Dash Target` 0.0))
  (bind _closest_actor (`local.Closest Actor`))
  (bind _returnvalue (select `bool` _tryingtomove :`false` 50.0 :`true` Range))
  (set `local.Closest Actor` null)
  (bind _output_get (set `local.Direction` _location))
  ;[0.09375 0.09375 0.09375] Find pawns in area ahead
  (set `local.Closeness` 0.0) ; reset
  (bind _returnvalue_2 (+ (`Actor.K2_GetActorLocation` (`self.Character`)) (* _output_get _returnvalue)))
  (bind (_outhits _returnvalue_3) (`KismetSystemLibrary.BoxTraceMulti` :`Start` _returnvalue_2 :`End` _returnvalue_2 :`HalfSize` (`KismetMathLibrary.MakeVector` _returnvalue 80.0 _returnvalue) :`Orientation` (`KismetMathLibrary.MakeRotFromZ` (`local.Direction`)) :`TraceChannel` "TraceTypeQuery3" :`DrawTime` 1.0))
  (if _returnvalue_3
    (for _array_element _outhits
      (bind (_bblockinghit _binitialoverlap _time _distance _location_2 _impactpoint _normal _impactnormal _physmat _hitactor) (`GameplayStatics.BreakHitResult` _array_element))
      (bind _returnvalue_4 (`KismetMathLibrary.Dot_VectorVector` (`KismetMathLibrary.Normal` (- (`Actor.K2_GetActorLocation` _hitactor) (`Actor.K2_GetActorLocation` (`self.Character`)))) (`local.Direction`)))
      ;[0.2153 0.2153 0.2153] Choose closest one in terms of direction. (the one player is currently moving towards)
      (if (> _returnvalue_4 (`local.Closeness`))
        (set `local.Closeness` _returnvalue_4)
        (bind _output_get_2 (set `local.Closest Actor` _hitactor))))
    (`/Engine/EditorBlueprintResources/StandardMacros.IsValid` _output_get_2
      (:`Is Valid`
        ;[0.2 0.2 0.2] Another character in the way? Choose that character instead.
        (bind (_outhit _returnvalue_5) (`KismetSystemLibrary.LineTraceSingle` (`Actor.K2_GetActorLocation` (`self.Character`)) (`Actor.K2_GetActorLocation` _closest_actor) "TraceTypeQuery3"))
        (bind _returnvalue_6 (select `bool` _returnvalue_5 :`false` _closest_actor :`true` (`.HitActor` (`GameplayStatics.BreakHitResult` _outhit))))
        (return (`KismetSystemLibrary.IsValid` _returnvalue_6) _returnvalue_6 (`local.Direction`)))
      (:`Is Not Valid`
        (return false null (`local.Direction`))))
    (else
      (return false null (`local.Direction`)) ; None found
    )))