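; Base magic container in the campfire prop folder that stores spells and hands them back, reporting fire as its spell type.
; GainSpell refuses a spell that would exceed the MagicComponent's maximum charges, otherwise activates it, adds it to the SpellBook and raises the charge count.
; ActivateMagic calls MoveToContainer, unhides the spell actor and prints a debug string.
; UseSpell returns the result of the component's RemoveSpell.
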(event `Activate Magic`
  (params (Spell :type "CPP_Spell Object Reference"))
  (`self.MoveToContainer` Spell)
  (`self.SetActorHiddenInGame` Spell false)
  (`KismetSystemLibrary.PrintString` "IN CONTAINER"))

(fn `GainSpell`
  (params (Spell :type "CPP_Spell Object Reference"))
  (returns (ReturnValue :type Boolean))
  (bind _returnvalue (`self.GetCharges`))
  (bind _returnvalue_2 (`self.GetMaximumCharges`))
  (bind _returnvalue_3 (+ _returnvalue (`CPP_Spell.SpellCharges` Spell)))
  (if (< _returnvalue_2 _returnvalue_3)
    (return false)
    (else
      (`self.Activate Magic` Spell)
      (`KismetArrayLibrary.Array_Add` (`MagicSystemComponent.SpellBook` (`self.Magic Component`)) Spell)
      (set `MagicSystemComponent.CurrentCharges` _returnvalue_3 (`self.Magic Component`))
      (return true))))

(fn `GetCharges`
  (returns (ReturnValue :type "Float (single-precision)"))
  (return (`MagicSystemComponent.CurrentCharges` (`self.Magic Component`))))

(fn `GetMaximumCharges`
  (returns (ReturnValue :type "Float (single-precision)"))
  (return (`MagicSystemComponent.MaxCharges` (`self.Magic Component`))))

(fn `GetSpellType`
  (returns (ReturnValue :type "CPP_Spell Class Reference"))
  (return "/Game/SpellSystem/Spells/Source/BP_FireSpell.BP_FireSpell_C"))

(fn `UserConstructionScript`)

(fn `UseSpell`
  (returns (ReturnValue :type "CPP_Spell Object Reference"))
  (bind _returnvalue (`MagicSystemComponent.RemoveSpell` (`self.Magic Component`)))
  (return _returnvalue))