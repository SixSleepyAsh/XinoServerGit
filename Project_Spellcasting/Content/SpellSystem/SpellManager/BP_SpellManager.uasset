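; Spell manager Blueprint that periodically refills spell containers with spells drawn from a pool.
; On BeginPlay it caches its managed actors as containers and starts a looping one-second timer.
; Each tick of that timer finds non-full containers, reads each one's spell type, and hands it a matching pooled spell through message calls.
; When no valid spell comes back, it prints that the pool is empty.
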(event `self.ReceiveBeginPlay`
  (bind _returnvalue (`self.GetManagedActors`))
  (set `self.Containers` _returnvalue)
  (`KismetSystemLibrary.K2_SetTimer` null "Regenerate Containers" 1.0 true))

(event `Regenerate Containers`
  (bind _returnvalue (`self.GetNonFullContainers` (`self.Containers`)))
  (if (not (`KismetArrayLibrary.Array_IsEmpty` _returnvalue))
    (for _array_element _returnvalue
      (bind _returnvalue_2 (message `CPP_MagicSystemInterface.GetSpellType` _array_element))
      (bind _returnvalue_3 (`self.GetSpellFromPool` _returnvalue_2))
      (if (`KismetSystemLibrary.IsValid` _returnvalue_3)
        (message `CPP_MagicSystemInterface.GainSpell` _array_element _returnvalue_3)
        (else
          (`KismetSystemLibrary.PrintString` "Pool is empty"))))))

(fn `UserConstructionScript`)