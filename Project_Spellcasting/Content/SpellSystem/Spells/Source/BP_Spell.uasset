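; Pooled spell projectile that homes in on the player and grants itself on overlap.
; Homing enables query collision, targets the player's HT2 component, starts the ribbon trail and moves above the current container target.
; Overlap calls GainSpell, hides and attaches the visual to HT2 while the trail fades, then spawns a received effect and resets.
; DestroySpell resets and returns it to SpellPool; the old hit-damage logic is disconnected.
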(event `self.Collision.OnComponentHit`
  (params (HitComponent :type "PrimitiveComponent Object Reference") (OtherActor :type "Actor Object Reference") (OtherComp :type "PrimitiveComponent Object Reference") (NormalImpulse :type "Vector Structure") (Hit :type "HitResult Structure (by ref)"))
  ;[0 0 0] attack (old)
)

(event `Homing`
  (bind _projectilemovementcomponent (`self.ProjectileMovementComponent`))
  ;[1 1 1] activate homing on F press (+teleport above source)
  (`PrimitiveComponent.SetCollisionEnabled` (`self.Collision`) "QueryOnly")
  (`ActorComponent.Activate` _projectilemovementcomponent false)
  (bind _asbp_temp_player (cast `/Game/ThirdPerson/Blueprints/BP_TempPlayer` (`GameplayStatics.GetPlayerCharacter` 0)))
  (set `ProjectileMovementComponent.HomingTargetComponent` (`/Game/ThirdPerson/Blueprints/BP_TempPlayer.HT2` _asbp_temp_player) _projectilemovementcomponent)
  (bind (_returnvalue_x _returnvalue_y _returnvalue_z) (`KismetMathLibrary.BreakVector` (`self.K2_GetActorLocation` (`Project_SpellcastingCharacter.CurrentContainerTarget` _asbp_temp_player))))
  (`AIBlueprintHelperLibrary.SimpleMoveToLocation` null (`KismetMathLibrary.MakeVector` _returnvalue_x _returnvalue_y (+ _returnvalue_z 200.0)))
  (`ActorComponent.Activate` (`self.ribbon`) false))

(event `self.Collision.OnComponentBeginOverlap`
  (params (OverlappedComponent :type "PrimitiveComponent Object Reference") (OtherActor :type "Actor Object Reference") (OtherComp :type "PrimitiveComponent Object Reference") (OtherBodyIndex :type Integer) (bFromSweep :type Boolean) (SweepResult :type "HitResult Structure (by ref)"))
  ;[1 1 1] give spell on player collision
  (bind _asbp_temp_player (cast `/Game/ThirdPerson/Blueprints/BP_TempPlayer` OtherActor))
  (`/Game/ThirdPerson/Blueprints/BP_TempPlayer.GainSpell` _asbp_temp_player self)
  (`KismetSystemLibrary.PrintString` "IN PLAYER")
  ;[1 1 1] hits target but sticks around while trail dies
  (`SceneComponent.SetVisibility` (`self.Visual`) false false)
  (`PrimitiveComponent.SetCollisionEnabled` (`self.Collision`) "NoCollision")
  (bind _asbp_temp_player_2 (cast `/Game/ThirdPerson/Blueprints/BP_TempPlayer` (`GameplayStatics.GetPlayerCharacter` 0)))
  (`SceneComponent.K2_AttachToComponent` (`self.Visual`) (`/Game/ThirdPerson/Blueprints/BP_TempPlayer.HT2` _asbp_temp_player_2) "None" "SnapToTarget" "SnapToTarget" "KeepRelative" true)
  (`KismetSystemLibrary.PrintString` "hit")
  ;[1 0.08248 0.1203] FOR MATERIAL TRANSITION
  (`KismetSystemLibrary.Delay` 0.3)
  (`NiagaraFunctionLibrary.SpawnSystemAttached` "/Game/SpellSystem/VFX/HomingParticle/NS_SpellReceived.NS_SpellReceived" (`/Game/ThirdPerson/Blueprints/BP_TempPlayer.HT2` _asbp_temp_player) "None" (0.0 0.0 0.0) (struct) "KeepRelativeOffset" true)
  ;[1 1 1] reset
  (`self.ResetProperties`)
  (`KismetSystemLibrary.PrintString` "SWITCHED"))

(event `self.ReceiveBeginPlay`
  ;[1 1 1] give spell on player collision
  (`PrimitiveComponent.SetCollisionEnabled` (`self.Collision`) "NoCollision"))

(event `Destroy Spell`
  ;[1 0 0.2195] Destroy the spell and return it to the spell pool
  (`self.ResetProperties`)
  (`CPP_SpellManager.ReturnSpellToPool` (`self.SpellPool`) self)
  (`KismetSystemLibrary.PrintString` "RETURNED"))

(fn `UserConstructionScript`)